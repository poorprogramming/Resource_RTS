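; Procedural mountain Blueprint that scatters static mesh components, placed entirely in the construction script with no active runtime logic.
; A seeded MountainRandomStream picks the component count, then gives each one a random X/Y offset within a small square at zero height.
; All components keep zero rotation and unit scale.
; Direction-vector nodes are left unconnected.
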(event EventBeginPlay)

(event Collision|EventActorBeginOverlap
  (params (OtherActor :type Actor%20Object%20Reference)))

(event EventTick
  (params (DeltaSeconds :type Float%20%28single-precision%29)))

(fn ConstructionScript
  (bind _mountain_randomstream (Variables|Default|GetMountain_RandomStream))
  (bind _output_get (Variables|Default|SetMountain_Range (Math|Random|RandomIntegerinRangefromStream 150 200 _mountain_randomstream)))
  (for _index (range 1 _output_get)
    (AddComponent|AddStaticMeshComponent false (Math|Transform|MakeTransform (Math|Vector|MakeVector (Math|Random|RandomFloatinRangefromStream 1.5e+02 2e+02 _mountain_randomstream) (Math|Random|RandomFloatinRangefromStream 1.5e+02 2e+02 _mountain_randomstream) 0.0)))))
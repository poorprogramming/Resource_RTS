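; Player commander pawn that provides a free-moving camera and controls for placing a source in game.
; On BeginPlay it shows the cursor, creates the UI_InGame HUD and registers both in ResourceGameInstance.
; Axis inputs move the actor, wheel or Space/Ctrl shifts InvisibleObject vertically as zoom, and right-mouse gates switch between pan and rotate via CameraTPanFRotate.
; While the HUD is placing, left click and Escape tell the GameMode to place or destroy the ghost.
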(event EventBeginPlay
  (CallFunction|StartUp))

(event EventTick
  (params (DeltaSeconds :type Float%20%28single-precision%29))
  (if (Variables|Orbits|GetInStrongOrbit)
    _))

(event Input|AxisEvents|InputAxisMoveForward
  (params (AxisValue :type Float%20%28single-precision%29))
  ;[1 1 1] Camera Directional Movement
  (Utilities|CameraMoveDirections AxisValue (stale Input|AxisEvents|InputAxisMoveRight AxisValue) (stale Input|AxisEvents|InputAxisMoveUp AxisValue)))

(event Input|AxisEvents|InputAxisMoveRight
  (params (AxisValue :type Float%20%28single-precision%29))
  ;[1 1 1] Camera Directional Movement
  (Utilities|CameraMoveDirections (stale Input|AxisEvents|InputAxisMoveForward AxisValue) AxisValue (stale Input|AxisEvents|InputAxisMoveUp AxisValue)) ; enters at LeftAndRight
)

(event Input|AxisEvents|InputAxisMoveUp
  (params (AxisValue :type Float%20%28single-precision%29))
  ;[1 1 1] Camera Directional Movement
  (Utilities|CameraMoveDirections (stale Input|AxisEvents|InputAxisMoveForward AxisValue) (stale Input|AxisEvents|InputAxisMoveRight AxisValue) AxisValue) ; enters at UpAndDown
)

(event Input|MouseEvents|MouseX
  (params (AxisValue :type Float%20%28single-precision%29))
  ;[1 1 1] Camera Pan/Rotate
  (Utilities|FlowControl|Gate true
    (:Exit
      (if (Variables|CameraMovements|GetCamera_TPanFRotate)
        (Utilities|CameraPan AxisValue (stale Input|MouseEvents|MouseY AxisValue))
        (else
          (Utilities|CameraRotate AxisValue (stale Input|MouseEvents|MouseY AxisValue)))))))

(event Input|MouseEvents|MouseY
  (params (AxisValue :type Float%20%28single-precision%29))
  ;[1 1 1] Camera Pan/Rotate
  (Utilities|FlowControl|Gate true
    (:Exit
      (if (Variables|CameraMovements|GetCamera_TPanFRotate)
        (Utilities|CameraPan (stale Input|MouseEvents|MouseX AxisValue) AxisValue) ; enters at MouseY
        (else
          (Utilities|CameraRotate (stale Input|MouseEvents|MouseX AxisValue) AxisValue) ; enters at MouseY
        )))))

(event Input|MouseEvents|MouseWheelUp
  (params (Key :type Key%20Structure :default "AnyKey"))
  ;[1 1 1] Camera Zoom
  (:Pressed
    (Utilities|CameraZoom)))

(event Input|MouseEvents|MouseWheelDown
  (params (Key :type Key%20Structure :default "AnyKey"))
  ;[1 1 1] Camera Zoom
  (:Pressed
    (Utilities|CameraZoom) ; enters at MoveDown
  ))

(event Input|KeyboardEvents|Escape
  (params (Key :type Key%20Structure :default "AnyKey"))
  (:Pressed
    (bind _asui_in_game (Utilities|Casting|CastToUI_InGame (Variables|Resources|GetCommanderHUD)))
    (if (Variables|/Game/Blueprints/UI_(Best_Folder)/UI_InGame.UI_InGame_C|GetPlacingSource _asui_in_game)
      (Class|ResourceInterface|DestroyGhost(Message) (Game|GetGameMode)))))

(event Input|MouseEvents|LeftMouseButton
  (params (Key :type Key%20Structure :default "AnyKey"))
  (:Pressed
    (bind _asui_in_game (Utilities|Casting|CastToUI_InGame (Variables|Resources|GetCommanderHUD)))
    (if (Variables|/Game/Blueprints/UI_(Best_Folder)/UI_InGame.UI_InGame_C|GetPlacingSource _asui_in_game)
      (Class|ResourceInterface|SourcePlaced(Message) (Game|GetGameMode)))))

(event Input|KeyboardEvents|LeftCtrl
  (params (Key :type Key%20Structure :default "AnyKey"))
  ;[1 1 1] Camera Zoom
  (:Pressed
    (Utilities|CameraZoom) ; enters at MoveDown
  ))

(event Input|KeyboardEvents|SpaceBar
  (params (Key :type Key%20Structure :default "AnyKey"))
  ;[1 1 1] Camera Zoom
  (:Pressed
    (Utilities|CameraZoom)))

(event Input|MouseEvents|RightMouseButton
  (params (Key :type Key%20Structure :default "AnyKey"))
  ;[1 1 1] Camera Pan/Rotate
  (:Pressed
    (Utilities|FlowControl|Sequence
      (:then_0
        (Utilities|FlowControl|Gate true) ; enters at Open
      )
      (:then_1
        (Utilities|FlowControl|Gate true) ; enters at Open
      )))
  (:Released
    (Utilities|FlowControl|Sequence
      (:then_0
        (Utilities|FlowControl|Gate true) ; enters at Close
      )
      (:then_1
        (Utilities|FlowControl|Gate true) ; enters at Close
      ))))

(fn ConstructionScript)

(fn StartUp
  (Variables|/Script/Engine.PlayerController|SetbShowMouseCursor (Game|GetPlayerController 0) true)
  (CallFunction|CreateWidgets)
  (CallFunction|SetGameInstanceVariable))

(fn CreateWidgets
  (bind _returnvalue (UserInterface|CreateWidget "/Game/Blueprints/UI_(Best_Folder)/UI_InGame.UI_InGame_C" 0 self))
  (bind _output_get (Variables|Resources|SetCommanderHUD _returnvalue))
  (bind _asresource_game_instance (Utilities|Casting|CastToResourceGameInstance (Game|GetGameInstance)))
  (bind _output_get_2 (Variables|/Game/Blueprints/Logic/ResourceGameInstance.ResourceGameInstance_C|SetCommanderHUD _asresource_game_instance _output_get))
  (UserInterface|Viewport|AddtoViewport _output_get_2 0))

(fn SetGameInstanceVariable
  (bind _asresource_game_instance (Utilities|Casting|CastToResourceGameInstance (Game|GetGameInstance)))
  (Variables|/Game/Blueprints/Logic/ResourceGameInstance.ResourceGameInstance_C|SetCommander _asresource_game_instance self)
  (Variables|/Game/Blueprints/Logic/ResourceGameInstance.ResourceGameInstance_C|SetCommanderHUD _asresource_game_instance (Variables|Resources|GetCommanderHUD)))
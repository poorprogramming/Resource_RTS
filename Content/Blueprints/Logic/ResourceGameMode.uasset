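; ResourceGameMode is a game mode Blueprint that spawns player pawns and acts as an event hub for the resource UI.
; SpawnPlayerCharacter spawns the given pawn class at a transform and has the supplied controller possess it.
; The other events forward resource button clicks, source placement, ghost destruction and durability updates straight to UIInGame, which is not assigned in these graphs.
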(event Custom|SpawnPlayerCharacter
  (params (InPawn :type Pawn%20Class%20Reference) (InSpawnTransform :type Transform) (InController :type Resource%20Player%20Controller%20Object%20Reference))
  (bind _returnvalue (Game|SpawnActorfromClass InPawn InSpawnTransform "Undefined" 0 0))
  (Pawn|Possess InController _returnvalue))

(event EventSourcePlaced
  ;[1 1 1] GhostSourceFollowMouse
  (Default|SourcePlaced (Variables|Resources|GetUI_InGame)))

(event EventDestroyGhost
  ;[1 1 1] GhostSourceFollowMouse
  (Default|DestroyGhost (Variables|Resources|GetUI_InGame)))

(event EventRSingleButton
  (params (ButtonInstructions :type String) (ClickedResourceSingle :type Resource%20Single%20Object%20Reference))
  (Default|RSingleButtonClicked (Variables|Resources|GetUI_InGame) ButtonInstructions ClickedResourceSingle))

(event EventUpdateDurability
  (params (InputResourceSingle :type Resource%20Single%20Object%20Reference))
  (Default|CEUpdateDurability (Variables|Resources|GetUI_InGame) InputResourceSingle))

(event EventRInfoButton
  (Default|RInfoButtonClicked (Variables|Resources|GetUI_InGame)))

(fn ConstructionScript)
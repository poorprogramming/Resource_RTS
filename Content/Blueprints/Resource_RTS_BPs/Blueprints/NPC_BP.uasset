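; NPC Blueprint that gives each character a random race, body color and name.
; The Construction Script creates a dynamic material on the mesh, tints it by race and stores name and race in NPCProfile.
; A nested branch chain rerolls the race at every test, so odds are uneven and all tests can fail.
; GetRandomName ANDs mutually exclusive race checks, so it always draws from the female name enum.
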(event EventBeginPlay)

(event Collision|EventActorBeginOverlap
  (params (OtherActor :type Actor%20Object%20Reference)))

(event EventTick
  (params (DeltaSeconds :type Float%20%28single-precision%29)))

(fn ConstructionScript
  (CallFunction|RandomNPCFeatures))

(fn RandomNPCFeatures
  (bind _returnvalue (Math|Random|RandomIntegerinRange 0 8))
  (bind _returnvalue_2 (Math|Conversions|ToByte(Integer) _returnvalue))
  (bind _returnvalue_3 (Utilities|Enum|ByteToEnumNPCRace_Enum _returnvalue_2))
  (bind _returnvalue_4 (Utilities|Enum|LiteralenumNPCRace_Enum _returnvalue_3))
  (bind _returnvalue_5 (Rendering|Material|CreateDynamicMaterialInstance (Variables|Character|GetMesh) 0 "/Game/Materials/Homo_Materials/HomoTexture_Mat_Inst.HomoTexture_Mat_Inst" :!class /Script/Engine.PrimitiveComponent))
  (LocalVariables|SetMaterialInstance _returnvalue_5)
  (if (Utilities|Enum|Equal(Enum) _returnvalue_4 "NewEnumerator0")
    (Rendering|Material|SetVectorParameterValue (LocalVariables|GetMaterialInstance) "BodyColor" (LocalVariables|GetOrcColor) :!class /Script/Engine.MaterialInstanceDynamic)
    (bind _name (CallFunction|GetRandomName "NewEnumerator0"))
    (Variables|Default|SetNPCProfile (Utilities|Struct|MakeNPCProfileStruct _name "NewEnumerator0"))
    (elif (Utilities|Enum|Equal(Enum) _returnvalue_4 "NewEnumerator1")
      (Rendering|Material|SetVectorParameterValue (LocalVariables|GetMaterialInstance) "BodyColor" (LocalVariables|GetBarbarianColor) :!class /Script/Engine.MaterialInstanceDynamic)
      (bind _name_2 (CallFunction|GetRandomName "NewEnumerator1"))
      (Variables|Default|SetNPCProfile (Utilities|Struct|MakeNPCProfileStruct _name_2 "NewEnumerator1"))
      (elif (Utilities|Enum|Equal(Enum) _returnvalue_4 "NewEnumerator2")
        (Rendering|Material|SetVectorParameterValue (LocalVariables|GetMaterialInstance) "BodyColor" (LocalVariables|GetHomoColor) :!class /Script/Engine.MaterialInstanceDynamic)
        (bind _name_3 (CallFunction|GetRandomName "NewEnumerator2"))
        (Variables|Default|SetNPCProfile (Utilities|Struct|MakeNPCProfileStruct _name_3 "NewEnumerator2"))
        (elif (Utilities|Enum|Equal(Enum) _returnvalue_4 "NewEnumerator3")
          (Rendering|Material|SetVectorParameterValue (LocalVariables|GetMaterialInstance) "BodyColor" (LocalVariables|GetElfColor) :!class /Script/Engine.MaterialInstanceDynamic)
          (bind _name_4 (CallFunction|GetRandomName "NewEnumerator3"))
          (Variables|Default|SetNPCProfile (Utilities|Struct|MakeNPCProfileStruct _name_4 "NewEnumerator3"))
          (elif (Utilities|Enum|Equal(Enum) _returnvalue_4 "NewEnumerator4")
            (Rendering|Material|SetVectorParameterValue (LocalVariables|GetMaterialInstance) "BodyColor" (LocalVariables|GetHobbitColor) :!class /Script/Engine.MaterialInstanceDynamic)
            (bind _name_5 (CallFunction|GetRandomName "NewEnumerator4"))
            (Variables|Default|SetNPCProfile (Utilities|Struct|MakeNPCProfileStruct _name_5 "NewEnumerator4"))
            (elif (Utilities|Enum|Equal(Enum) _returnvalue_4 "NewEnumerator5")
              (Rendering|Material|SetVectorParameterValue (LocalVariables|GetMaterialInstance) "BodyColor" (LocalVariables|GetUndeadColor) :!class /Script/Engine.MaterialInstanceDynamic)
              (bind _name_6 (CallFunction|GetRandomName "NewEnumerator5"))
              (Variables|Default|SetNPCProfile (Utilities|Struct|MakeNPCProfileStruct _name_6 "NewEnumerator5"))
              (elif (Utilities|Enum|Equal(Enum) _returnvalue_4 "NewEnumerator6")
                (Rendering|Material|SetVectorParameterValue (LocalVariables|GetMaterialInstance) "BodyColor" (LocalVariables|GetWizardColor) :!class /Script/Engine.MaterialInstanceDynamic)
                (bind _name_7 (CallFunction|GetRandomName "NewEnumerator6"))
                (Variables|Default|SetNPCProfile (Utilities|Struct|MakeNPCProfileStruct _name_7 "NewEnumerator6"))
                (elif (Utilities|Enum|Equal(Enum) _returnvalue_4 "NewEnumerator7")
                  (Rendering|Material|SetVectorParameterValue (LocalVariables|GetMaterialInstance) "BodyColor" (LocalVariables|GetDwarfColor) :!class /Script/Engine.MaterialInstanceDynamic)
                  (bind _name_8 (CallFunction|GetRandomName "NewEnumerator7"))
                  (Variables|Default|SetNPCProfile (Utilities|Struct|MakeNPCProfileStruct _name_8 "NewEnumerator7"))
                  (elif (Utilities|Enum|Equal(Enum) _returnvalue_4 "NewEnumerator8")
                    (Rendering|Material|SetVectorParameterValue (LocalVariables|GetMaterialInstance) "BodyColor" (LocalVariables|GetAlienColor) :!class /Script/Engine.MaterialInstanceDynamic)
                    (bind _name_9 (CallFunction|GetRandomName "NewEnumerator8"))
                    (Variables|Default|SetNPCProfile (Utilities|Struct|MakeNPCProfileStruct _name_9 "NewEnumerator8"))))))))))))

(fn GetRandomName
  (params (Race :type NPCRace_Enum%20Enum :default "NewEnumerator0"))
  (if (Math|Boolean|ANDBoolean (Utilities|Enum|Equal(Enum) Race "NewEnumerator0") (Utilities|Enum|Equal(Enum) Race "NewEnumerator1") (Utilities|Enum|Equal(Enum) Race "NewEnumerator2") (Utilities|Enum|Equal(Enum) Race "NewEnumerator5") (Utilities|Enum|Equal(Enum) Race "NewEnumerator7") (Utilities|Enum|Equal(Enum) Race "NewEnumerator6"))
    (return (Utilities|String|EnumtoString (Utilities|Enum|LiteralenumNPCNameMaleHomo_Enum (Utilities|Enum|ByteToEnumNPCNameMaleHomo_Enum (Math|Conversions|ToByte(Integer) (Math|Random|RandomIntegerinRange 0 (- (|GetNumEnumEntries) 1)))))))
    (else
      (return (Utilities|String|EnumtoString (Utilities|Enum|LiteralenumNPCNameFemaleHomo_Enum (Utilities|Enum|ByteToEnumNPCNameFemaleHomo_Enum (Math|Conversions|ToByte(Integer) (Math|Random|RandomIntegerinRange 0 (- (|GetNumEnumEntries) 1))))))))))
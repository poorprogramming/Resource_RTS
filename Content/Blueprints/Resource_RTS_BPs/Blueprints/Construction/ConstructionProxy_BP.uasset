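; Construction-site placeholder actor for the RTS that shows a ghost-material building mesh while workers build it.
; Each tick with workers assigned, it advances a build clock using the game-speed time unit divided by worker count.
; Workers register through ReportToShift, and game-speed changes update the time unit via a GameState binding.
; When the required time elapses, it signals completion, frees and unhides the workers, then destroys itself after a short delay.
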(event Custom|AdjustTime
  (params (TimeUnit :type Float%20%28single-precision%29))
  (Variables|Time|SetTimeUnit TimeUnit))

(event EventBeginPlay
  (bind _output_get (Variables|References|SetGameStateRef (.AsRRTSGame%20State%20Base (Utilities|Casting|CastToRRTSGameStateBase (Game|GetGameState)))))
  (EventDispatchers|BindEventtoUpdateGameSpeed _output_get (EventDispatchers|CreateEvent :!event Custom|AdjustTime))
  (bind _timeunit (Default|GetCurrentTimeUnit (Variables|References|GetGameStateRef)))
  (Variables|Time|SetTimeUnit _timeunit))

(event EventTick
  (params (DeltaSeconds :type Float%20%28single-precision%29))
  (Variables|Time|SetDelta DeltaSeconds)
  (if (not (Variables|Default|GetIsConstructionCompleted))
    (CallFunction|DoBuild)
    (if (>= (Variables|Default|GetBuildTimeSpent) (Variables|Default|GetHomoHours))
      (Variables|Default|SetIsConstructionCompleted true)
      (Default|CallConstructionCompleted self)
      (CallFunction|SourceComplete)
      (Utilities|FlowControl|Delay 0.2)
      (Actor|DestroyActor))))

(fn ConstructionScript
  (bind _staticmesh (Variables|Default|GetStaticMesh))
  (Components|StaticMesh|SetStaticMesh _staticmesh (Variables|Default|GetDisplayMesh))
  (Rendering|Material|SetMaterialbyName _staticmesh "Baseplate" "/Game/Blueprints/Materials/Ghost_M_Inst.Ghost_M_Inst")
  (Rendering|Material|SetMaterialbyName _staticmesh "Grass" "/Game/Blueprints/Materials/Ghost_M_Inst.Ghost_M_Inst")
  (Transformation|SetWorldScale3D _staticmesh "4.000000,4.000000,4.000000")
  (CallFunction|SetSourceEntrance (Variables|Default|GetEntrance) (Variables|Default|GetStaticMesh))
  (CallFunction|SetSourceCollisionBox (Variables|Default|GetCollision) (Variables|Default|GetStaticMesh)))

(fn SetConstructionTime
  (params (BuildTime :type Float%20%28single-precision%29))
  (Variables|Default|SetHomoHours (* BuildTime 6e+01))
  (return))

(fn DoBuild
  (bind _activeworkers (CallFunction|GetWorkforce))
  (if (> _activeworkers 0.0)
    (bind _output_get (Variables|Time|SetClockwork (.ClockworkOut (CallFunction|SetClockwork (Variables|Time|GetDelta) (/ (Variables|Time|GetTimeUnit) _activeworkers) (Variables|Time|GetClockwork)))))
    (Variables|Default|SetBuildTimeSpent (* _output_get 6e+01))
    (return)
    (else
      (return))))

(fn GetWorkforce
  (return (Math|Conversions|ToFloat(Integer) (Utilities|Array|Length (Variables|Default|GetActiveWorkers)))))

(fn ReporttoShift
  (params (Worker :type NPC%20BP%20Object%20Reference))
  (Utilities|Array|Add (Variables|Default|GetActiveWorkers) Worker)
  (return))

(fn SourceComplete
  (if (> (CallFunction|GetWorkforce) 0.0)
    (for _array_element (Variables|Default|GetActiveWorkers)
      (Default|SetIsBusy _array_element false)
      (Rendering|SetActorHiddenInGame _array_element false))
    (Variables|Default|SetActiveWorkers (Utilities|Array|MakeArray 0))
    (return)
    (else
      (return))))
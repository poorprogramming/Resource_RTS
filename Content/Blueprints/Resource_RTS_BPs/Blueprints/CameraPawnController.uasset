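; Player controller for an RTS that drives the camera pawn and handles ghost-based building placement.
; BeginPlay spawns the construction manager and ghost source, then creates the in-game HUD.
; Input moves, pans, zooms and edge-scrolls the camera, with Shift boosting movement and key-move speed scaling with zoom.
; In build mode, Tick moves the ghost to the cursor, keys rotate it, and left-click queues non-overlapping placements with the manager.
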(event EventBeginPlay
  (bind _returnvalue (Math|Transform|MakeTransform "0, 0, 0" "0, 0, 0" "4.000000,4.000000,4.000000"))
  ;[1 1 1] Begin Play
  (Utilities|FlowControl|Sequence
    (:then_0
      (Utilities|ReferenceCasts))
    (:then_1
      (bind _returnvalue_2 (Game|SpawnActorfromClass "/Game/Blueprints/Resource_RTS_BPs/Blueprints/Construction/ConstructionManager_BP.ConstructionManager_BP_C" _returnvalue "AlwaysSpawn" 0 0))
      (Variables|Referances|SetConstructionManagerRef _returnvalue_2))
    (:then_2
      (bind _returnvalue_3 (Game|SpawnActorfromClass "/Game/Blueprints/Resource_RTS_BPs/Blueprints/Sources/GhostSource_BP.GhostSource_BP_C" _returnvalue "AlwaysSpawn" 0 self 0))
      (Variables|Referances|SetGhostSourceRef _returnvalue_3))
    (:then_3
      (Input|SetInputModeGameandUI self 0 "LockAlways" false)
      (Utilities|CreateHuds)
      (UserInterface|Viewport|AddtoViewport (Variables|Referances|GetUI_InGameRef) 0))))

(event EventTick
  (params (DeltaSeconds :type Float%20%28single-precision%29))
  (if (Variables|Default|GetBuildModeActive)
    (|SetCursorWorldPosition)))

(event Input|ActionEvents|InputActionPan
  (params (Key :type Key%20Structure))
  (bind _camerapawnref (Variables|Referances|GetCameraPawnRef))
  (bind _returnvalue (Transformation|GetActorRotation _camerapawnref))
  (bind (_roll _pitch _yaw) (Math|Rotator|BreakRotator _returnvalue))
  ;[1 1 1] Camera Movement
  ;;[1 1 1] Pan Y
  (:Pressed
    (Variables|Default|SetDisableCamNav true)
    (Utilities|FlowControl|Gate true) ; enters at Open
  )
  (:Released
    (Variables|Default|SetDisableCamNav false)
    (Utilities|FlowControl|Gate true) ; enters at Close
  ))

(event Input|ActionEvents|InputActionDeSelect
  (params (Key :type Key%20Structure))
  (:Pressed
    (if (Variables|Default|GetBuildModeActive)
      (Default|KillGhost (Variables|Referances|GetGhostSourceRef))
      (Variables|Default|SetBuildModeActive false))))

(event Input|ActionEvents|InputActionPan
  (params (Key :type Key%20Structure))
  (bind _camerapawnref (Variables|Referances|GetCameraPawnRef))
  (bind _returnvalue (Transformation|GetActorRotation _camerapawnref))
  (bind (_roll _pitch _yaw) (Math|Rotator|BreakRotator _returnvalue))
  ;[1 1 1] Camera Movement
  ;;[1 1 1] Pan Z
  (:Pressed
    (Variables|Default|SetDisableCamNav true)
    (Utilities|FlowControl|Gate true) ; enters at Open
  )
  (:Released
    (Variables|Default|SetDisableCamNav false)
    (Utilities|FlowControl|Gate true) ; enters at Close
  ))

(event Input|ActionEvents|InputActionRotateSourceRight
  (params (Key :type Key%20Structure))
  (bind _ghostsourceref (Variables|Referances|GetGhostSourceRef))
  (bind _returnvalue (Transformation|GetActorRotation _ghostsourceref))
  (bind (_roll _pitch _yaw) (Math|Rotator|BreakRotator _returnvalue))
  ;[1 1 1] Left Mouse Button
  (:Pressed
    (if (and (Utilities|IsValid _ghostsourceref) (Variables|Default|GetBuildModeActive))
      (Transformation|SetActorRotation _ghostsourceref (Math|Rotator|MakeRotator _roll _pitch (- _yaw (Variables|Default|GetSourceRotationRate)))))))

(event Input|ActionEvents|InputActionRotateSourceLeft
  (params (Key :type Key%20Structure))
  (bind _ghostsourceref (Variables|Referances|GetGhostSourceRef))
  (bind _returnvalue (Transformation|GetActorRotation _ghostsourceref))
  (bind (_roll _pitch _yaw) (Math|Rotator|BreakRotator _returnvalue))
  ;[1 1 1] Left Mouse Button
  (:Pressed
    (if (and (Utilities|IsValid _ghostsourceref) (Variables|Default|GetBuildModeActive))
      (Transformation|SetActorRotation _ghostsourceref (Math|Rotator|MakeRotator _roll _pitch (+ _yaw (Variables|Default|GetSourceRotationRate)))))))

(event Input|ActionEvents|InputActionPanReset
  (params (Key :type Key%20Structure))
  (bind _camerapawnref (Variables|Referances|GetCameraPawnRef))
  (bind _returnvalue (Transformation|GetActorRotation _camerapawnref))
  (bind (_roll _pitch _yaw) (Math|Rotator|BreakRotator _returnvalue))
  ;[1 1 1] Camera Movement
  ;;[1 1 1] Pan Reset
  (:Pressed
    (Transformation|SetActorRotation _camerapawnref (Math|Rotator|MakeRotator _roll 0.0 _yaw))))

(event Input|ActionEvents|InputActionZoomReset
  (params (Key :type Key%20Structure))
  ;[1 1 1] Camera Movement
  ;;[1 1 1] Zoom Reset
  (:Pressed
    (Variables|/Script/Engine.SpringArmComponent|SetTargetArmLength (Variables|/Game/Blueprints/Resource_RTS_BPs/Blueprints/CameraPawn.CameraPawn_C|GetSpringArm (Variables|Referances|GetCameraPawnRef)) 1.5e+03)))

(event Input|ActionEvents|InputActionZoomIn
  (params (Key :type Key%20Structure))
  (bind _camerapawnref (Variables|Referances|GetCameraPawnRef))
  (bind _springarm (Variables|/Game/Blueprints/Resource_RTS_BPs/Blueprints/CameraPawn.CameraPawn_C|GetSpringArm _camerapawnref))
  ;[1 1 1] Camera Movement
  ;;[1 1 1] Zoom In/Out
  (:Pressed
    (Variables|/Script/Engine.SpringArmComponent|SetTargetArmLength _springarm (Math|Float|Clamp(Float) (- (Variables|/Script/Engine.SpringArmComponent|GetTargetArmLength _springarm) (Variables|Default|GetZoomSensitivity)) 5e+02 (Variables|Default|GetMaxArmDistance)))))

(event Input|ActionEvents|InputActionZoomOut
  (params (Key :type Key%20Structure))
  (bind _camerapawnref (Variables|Referances|GetCameraPawnRef))
  (bind _springarm (Variables|/Game/Blueprints/Resource_RTS_BPs/Blueprints/CameraPawn.CameraPawn_C|GetSpringArm _camerapawnref))
  ;[1 1 1] Camera Movement
  ;;[1 1 1] Zoom In/Out
  (:Pressed
    (Variables|/Script/Engine.SpringArmComponent|SetTargetArmLength _springarm (Math|Float|Clamp(Float) (+ (Variables|Default|GetZoomSensitivity) (Variables|/Script/Engine.SpringArmComponent|GetTargetArmLength _springarm)) 5e+02 (Variables|Default|GetMaxArmDistance)))))

(event Input|AxisEvents|InputAxisMoveForward
  (params (AxisValue :type Float%20%28single-precision%29))
  ;[1 1 1] Camera Movement
  ;;[1 1 1] Movement X
  (if (not (Variables|Default|GetDisableCamNav))
    (Transformation|SetActorTransform (Variables|Referances|GetCameraPawnRef) (Utilities|MovementX (CallFunction|MovementSpeedCalculation) (Variables|Default|GetFastMoveMultiplier) AxisValue (Variables|Referances|GetCameraPawnRef)))))

(event Input|AxisEvents|InputAxisMoveRight
  (params (AxisValue :type Float%20%28single-precision%29))
  (bind _movesensitivity (CallFunction|MovementSpeedCalculation))
  (bind _fastmovemultiplier (Variables|Default|GetFastMoveMultiplier))
  (bind _camerapawnref (Variables|Referances|GetCameraPawnRef))
  (bind _transform (Utilities|MovementY AxisValue _movesensitivity _fastmovemultiplier _camerapawnref))
  (bind (_location _rotation _scale) (Math|Transform|BreakTransform _transform))
  (bind (_x _y) (Math|Vector|BreakVector _location))
  ;[1 1 1] Camera Movement
  ;;[1 1 1] Movement Y
  (if (not (Variables|Default|GetDisableCamNav))
    (Transformation|SetActorTransform (Variables|Referances|GetCameraPawnRef) (Math|Transform|MakeTransform (Math|Vector|MakeVector _x _y 1e+02) _rotation _scale))))

(event Input|MouseEvents|MouseX
  (params (AxisValue :type Float%20%28single-precision%29))
  (bind _camerapawnref (Variables|Referances|GetCameraPawnRef))
  (bind _returnvalue (Transformation|GetActorRotation _camerapawnref))
  (bind (_roll _pitch _yaw) (Math|Rotator|BreakRotator _returnvalue))
  ;[1 1 1] Camera Movement
  ;;[1 1 1] Pan Z
  (Utilities|FlowControl|Gate true
    (:Exit
      (Transformation|SetActorRotation (Variables|Referances|GetCameraPawnRef) (Math|Rotator|MakeRotator _roll _pitch (+ _yaw (* (Variables|Default|GetPanSensitivity) AxisValue)))))))

(event Input|MouseEvents|MouseY
  (params (AxisValue :type Float%20%28single-precision%29))
  (bind _camerapawnref (Variables|Referances|GetCameraPawnRef))
  (bind _returnvalue (Transformation|GetActorRotation _camerapawnref))
  (bind (_roll _pitch _yaw) (Math|Rotator|BreakRotator _returnvalue))
  ;[1 1 1] Camera Movement
  ;;[1 1 1] Pan Y
  (Utilities|FlowControl|Gate true
    (:Exit
      (Transformation|SetActorRotation (Variables|Referances|GetCameraPawnRef) (Math|Rotator|MakeRotator _roll (Math|Float|Clamp(Float) (+ _pitch (* (Variables|Default|GetPanSensitivity) AxisValue)) -15.0 45.0) _yaw)))))

(event Input|MouseEvents|MouseX
  (params (AxisValue :type Float%20%28single-precision%29))
  ;[1 1 1] Camera Movement
  ;;[1 1 1] Edge Movement
  (if (not (Variables|Default|GetDisableCamNav))
    (bind (_deltaxspeed _deltayspeed) (Utilities|ScreenEdgeMovement))
    (Transformation|AddActorLocalOffset (Variables|Referances|GetCameraPawnRef) (Math|Vector|MakeVector _deltaxspeed _deltayspeed 0.0) true false)))

(event Input|MouseEvents|MouseY
  (params (AxisValue :type Float%20%28single-precision%29))
  ;[1 1 1] Camera Movement
  ;;[1 1 1] Edge Movement
  (if (not (Variables|Default|GetDisableCamNav))
    (Utilities|ScreenEdgeMovement) ; enters at MouseY
  ))

(event Input|KeyboardEvents|LeftShift
  (params (Key :type Key%20Structure))
  ;[1 1 1] Camera Movement
  ;;[1 1 1] Move Multiplier
  (:Pressed
    (Variables|Default|SetFastMoveMultiplier 5.0))
  (:Released
    (Variables|Default|SetFastMoveMultiplier 1.0)))

(event Input|MouseEvents|LeftMouseButton
  (params (Key :type Key%20Structure))
  ;[1 1 1] Left Mouse Button
  (:Pressed
    (if (|VerifyAsPlaceable)
      (bind _constructionstruct (Default|GetConstructionStruct (Variables|Referances|GetGhostSourceRef)))
      (Default|QueueConstruction (Variables|Referances|GetConstructionManagerRef) _constructionstruct)
      (Default|KillGhost (Variables|Referances|GetGhostSourceRef)))))

(fn ConstructionScript)

(fn MovementSpeedCalculation
  (return (Math|Float|Clamp(Float) (/ (Variables|/Script/Engine.SpringArmComponent|GetTargetArmLength (Variables|/Game/Blueprints/Resource_RTS_BPs/Blueprints/CameraPawn.CameraPawn_C|GetSpringArm (Variables|Referances|GetCameraPawnRef))) 1e+02) 5.0 2e+01)))

(fn SetSightDistance
  (return (+ (Variables|Default|GetSightDistance) (Variables|/Script/Engine.SpringArmComponent|GetTargetArmLength (Variables|/Game/Blueprints/Resource_RTS_BPs/Blueprints/CameraPawn.CameraPawn_C|GetSpringArm (Variables|Referances|GetCameraPawnRef))))))

(fn SetCalendar
  (params (Date :type Array%20of%20Integers))
  (return false))

(fn SetClock
  (params (Time :type Array%20of%20Integers))
  (return false))
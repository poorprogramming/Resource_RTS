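; GhostSource_BP is a poolable ghost actor that displays a mesh standing in for a source in the RTS resource system.
; OnSpawn, only when inactive, stores the display mesh, source age and construction proxy, marks itself active and applies the mesh to GhostSourceMesh.
; KillGhost clears the stored references and active flag for reuse, leaving the component's mesh unchanged.
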(event Custom|OnSpawn
  (params (DisplayMesh :type Static%20Mesh%20Object%20Reference) (SourceAge :type Source%20Master%20BP%20Class%20Reference) (ConstructionProxy :type Construction%20Proxy%20BP%20Class%20Reference))
  (if (not (Variables|Default|GetIsActive))
    (Variables|Default|SetSourceAge SourceAge)
    (Variables|Default|SetConstructionProxy ConstructionProxy)
    (Variables|Default|SetDisplayMesh DisplayMesh)
    (Variables|Default|SetIsActive true)
    (Components|StaticMesh|SetStaticMesh (Variables|Default|GetGhostSource_Mesh) (Variables|Default|GetDisplayMesh))))

(event Custom|KillGhost
  (Variables|Default|SetSourceAge 0)
  (Variables|Default|SetConstructionProxy 0)
  (Variables|Default|SetDisplayMesh 0)
  (Variables|Default|SetIsActive false))

(fn ConstructionScript)